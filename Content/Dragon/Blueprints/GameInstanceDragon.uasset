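; Game instance Blueprint for the Dragon game that handles in-app purchase restore and platform achievement writes.
; Restore results pass through a HandleIAPResult macro, whose body is empty, while HandleThemeSuccess flags the theme purchase and calls a save.
; WhiteArchievement writes progress to the platform, then mirrors it into a local array by index.
; Leaderboard and achievement caching exist only as disconnected nodes, and CheckArchievement is a stub.
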(event Custom|RestoreIAP
  (bind (_completionstatus _inapprestorepurchaseinformation) (|InAppPurchaseRestore (Utilities|Array|MakeArray "") (Game|GetPlayerController 0))
    (:OnSuccess
      _)
    (:OnFailure
      _))
  (Utilities|HandleIAPResult _completionstatus
    (:Success
      (if (Utilities|Enum|Equal(Enum) (.Identifier (Utilities|Struct|BreakInAppPurchaseRestoreInfo (Utilities|Array|Get(acopy) _inapprestorepurchaseinformation))) (Variables|Default|GetIAP%20Theme))
        _))))

(event Custom|WhiteArchievement
  (params (Archievement :type Name) (Progress :type Float%20%28single-precision%29) (Index :type Integer))
  ;[1 1 1] Whiting Values to your Archievement
  (bind (_writtenachievementname _writtenprogress _writtenusertag) (|WriteAchievementProgress (Game|GetPlayerController 0) Archievement Progress Index)
    (:OnSuccess
      (Development|PrintString (Utilities|String|BuildString(Float) "" (Utilities|String|BuildString(Name) "" "***Wrote to" _writtenachievementname "a value of:") _writtenprogress "***"))
      (Utilities|Array|SetArrayElem (Variables|Default|GetAchievement%20Progress) _writtenusertag _writtenprogress)
      (Utilities|Array|SetArrayElem (Variables|Default|GetAchievement%20Progress) _writtenusertag _writtenprogress true))))

(fn HandleThemeSuccess
  (params (Calling%20Widget :type Box%20Structure))
  ;[1 1 1] Comment
  (Variables|Default|SetTheme%20Purchase true)
  (Development|PrintString "Hello")
  (SaveGame|SaveGametoSlot)
  (if (not true)
    (Development|PrintString "***Handle Theme Not Called Fraom A Widget***")))

(fn CheckArchievement)