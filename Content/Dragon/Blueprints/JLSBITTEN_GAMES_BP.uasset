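; Actor named for JLSBITTEN Games, apparently part of a studio intro, that moves a static mesh and then brings in another level.
; On BeginPlay it plays the COMENDO sound at the world origin.
; Each Tick shifts the mesh along negative world X by a fixed, frame-rate-dependent step.
; Tick also runs a one-second Delay into a DoOnce, which loads JLSB3 as a level instance at the origin.
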(event EventBeginPlay
  (Audio|SpawnSoundatLocation "/Game/Dragon/Audio/COMENDO.COMENDO" "0, 0, 0"))

(event EventTick
  (params (DeltaSeconds :type Float%20%28single-precision%29))
  (Transformation|SetWorldLocation (Variables|Debug|GetStaticMeshComponent) (+ (Transformation|GetWorldLocation (Variables|Debug|GetStaticMeshComponent)) "-5.000000,0.000000,0.000000") false false)
  (Utilities|FlowControl|Delay 1.0)
  (Utilities|FlowControl|DoOnce false
    (:Completed
      (Class|LevelStreamingKismet|LoadLevelInstance "JLSB3" (Math|Vector|MakeVector 0.0 0.0 0.0) (Math|Rotator|MakeRotator 0.0 0.0 0.0)))))

(fn ConstructionScript)