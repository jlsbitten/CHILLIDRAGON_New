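; Pet dragon Blueprint that wanders randomly within a fixed area of the level.
; BeginPlay loops the Eating animation, commented as wing flapping, then reissues AI MoveTo every two seconds with a random box point, though Target Actor is wired to its own controller.
; Disconnected, never-run logic would send it to a fixed spot when ComendoRef's Comendo (eating) flag is set, alongside an alternative SimpleMoveToLocation wander.
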(event EventBeginPlay
  ;[1 1 1] Anda aleatóriamente
  ;[1 1 1] Bate asas desde inicio
  (Components|Animation|PlayAnimation (Variables|Default|GetPetDragon) "/Game/Dragon/Anim/Eating.Eating" true)
  (AI|AIMoveTo 0 (Math|Random|RandomPointinBoundingBox (Math|Vector|MakeVector 7649.0 3e+03 498.0) (Math|Vector|MakeVector 5e+02 2e+02 0.0)) (Pawn|GetController) 1.0 false :!label _label
    (:then
      (Utilities|FlowControl|Delay 2.0)
      (goto _label))))

(fn ConstructionScript)