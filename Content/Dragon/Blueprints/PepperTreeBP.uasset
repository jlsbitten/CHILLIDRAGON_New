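; PepperTreeBP is a collectible pepper tree that jumps to a random spot in a fixed area at a set height.
; InitPepper places it at BeginPlay and calls a timer on itself, though no interval is shown.
; Overlap with BP_DRAGON plays audio and, unless the game is over, reports the pickup to DragonHUD and relocates the tree.
; Ending the overlap stops the audio.
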(event Custom|InitPepper
  ;[1 1 1] Spawn in Scene
  (Transformation|SetActorLocation (Math|Vector|MakeVector (Math|Random|RandomFloatinRange 3e+03 4e+04) (Math|Random|RandomFloatinRange -2.3e+03 1e+04) 2.3e+02) false false)
  (Utilities|Time|SetTimerbyFunctionName 0 "InitPepper" 0.0))

(event EventTick
  (params (DeltaSeconds :type Float%20%28single-precision%29)))

(event Collision|EventActorEndOverlap
  (params (OtherActor :type Actor%20Object%20Reference))
  (Utilities|Casting|CastToBP_DRAGON OtherActor)
  (Audio|Components|Audio|Stop (Variables|Default|GetAudio)))

(event EventBeginPlay
  (bind _asdragon_hud (Utilities|Casting|CastToDragonHUD (HUD|GetHUD (Game|GetPlayerController 0))))
  (Variables|Default|SetDragonHUD _asdragon_hud)
  (CallFunction|InitPepper))

(event Collision|EventActorBeginOverlap
  (params (OtherActor :type Actor%20Object%20Reference))
  (Utilities|Casting|CastToBP_DRAGON OtherActor)
  (Audio|Components|Audio|Play (Variables|Default|GetAudio) 0.0)
  (if (not (Variables|/Game/Dragon/DragonHUD/Blueprints/DragonHUD.DragonHUD_C|GetGameOver (Variables|Default|GetDragonHUD)))
    (Default|PepperCollected (Variables|Default|GetDragonHUD))
    (CallFunction|InitPepper)))

(fn ConstructionScript)