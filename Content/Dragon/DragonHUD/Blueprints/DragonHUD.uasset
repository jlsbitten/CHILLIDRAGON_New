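; HUD Blueprint for a dragon pepper-collecting game that also owns the game state: score, countdown, level and pepper count.
; StartGame resets state and starts a looping Clock timer that triggers game over at zero; Enter restarts.
; PepperCollected adds level-scaled score and periodically grants time and a capped level-up, while DrawHUD renders stats and game-over text.
; P and L quick-save and load stats plus player and pepper tree transforms through a SaveInfo slot.
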(event Custom|Clock
  ;[1 1 1] Clock
  (Variables|Default|SetTime (- (Variables|Default|GetTime) 1))
  (if (== (Variables|Default|GetTime) 0)
    (Variables|Default|SetGameOver true)
    (Utilities|Time|ClearTimerbyFunctionName 0 "Clock")))

(event EventBeginPlay
  ;[1 1 1] Start GAME - Para funcionar input no HUD BP
  (Utilities|StartGame
    (:Out
      (Input|EnableInput (Game|GetPlayerController 0))
      (Audio|PlaySoundatLocation "/Game/Dragon/Audio/Ambient_Cave_Wind05.Ambient_Cave_Wind05" "0, 0, 0"))))

(event EventDrawHUD
  (params (SizeX :type Integer) (SizeY :type Integer))
  (bind _returnvalue (Viewport|GetViewportSize))
  (bind (_x _y) (Math|Vector2D|BreakVector2D _returnvalue))
  (bind _returnvalue_2 (/ _x 2.0))
  (bind _returnvalue_3 (* _y 0.015))
  (bind _returnvalue_4 (* _x 0.83))
  ;[1 1 1] Draw HUD
  (HUD|DrawText (Utilities|String|BuildString(Integer) "Score: " "" (Variables|Default|GetScore)) "(R=0.930000,G=0.861424,B=0.135878,A=1.000000)" (* _x 0.04) _returnvalue_3 0 3.0 false)
  (HUD|DrawText (Utilities|String|BuildString(Integer) "Time: " "" (Variables|Default|GetTime)) "(R=0.930000,G=0.116935,B=0.709305,A=1.000000)" (- _returnvalue_2 (/ 75.0 1.0)) _returnvalue_3 0 3.0 false)
  (HUD|DrawText (Utilities|String|BuildString(Integer) "Level: " "" (Variables|Default|GetLevel)) "(R=0.198158,G=0.930000,B=0.158584,A=1.000000)" _returnvalue_4 _returnvalue_3 0 3.0 false)
  (HUD|DrawText (Utilities|String|BuildString(Integer) "Peppers: " "" (Variables|Default|GetPepperCount)) "(R=0.009000,G=0.039943,B=0.450000,A=1.000000)" _returnvalue_4 (+ _returnvalue_3 55.0) 0 3.0 false)
  (if (Variables|Default|GetGameOver)
    (HUD|DrawText "GAME OVER" "(R=0.360000,G=0.014400,B=0.067463,A=1.000000)" (- _returnvalue_2 (/ (.OutWidth (Class|HUD|GetTextSize "GAMEOVER" 0 5.0)) 2.0)) 2e+02 0 5.0 false)
    (HUD|DrawText "PRESS ENTER" "(R=0.930000,G=0.027900,B=0.116977,A=1.000000)" (- _returnvalue_2 (/ (.OutWidth (Class|HUD|GetTextSize "PRESS ENTER" 0 3.0)) 2.0)) 3.5e+02 0 3.0 false)))

(event Input|KeyboardEvents|P
  (params (Key :type Key%20Structure :default "AnyKey"))
  ;[1 1 1] QuickSave
  (:Pressed
    (bind _returnvalue (SaveGame|CreateSaveGameObject "/Game/Dragon/Blueprints/SaveInfo.SaveInfo_C"))
    (bind _assave_info (Utilities|Casting|CastToSaveInfo _returnvalue))
    (Variables|Default|SetSaveInfoVar _assave_info)
    (Utilities|SaveGameVars)
    (Utilities|SaveTransform
      (:LoopBody
        (SaveGame|SaveGametoSlot (Variables|Default|GetSaveInfoVar) "BP_Game")))))

(event Input|KeyboardEvents|Enter
  (params (Key :type Key%20Structure :default "AnyKey"))
  ;[1 1 1] Start GAME - Para funcionar input no HUD BP
  (:Pressed
    (Utilities|StartGame
      (:Out
        (Audio|PlaySoundatLocation "/Game/Dragon/Audio/Ambient_Cave_Wind05.Ambient_Cave_Wind05" "0, 0, 0")))))

(event Input|KeyboardEvents|L
  (params (Key :type Key%20Structure :default "AnyKey"))
  ;[1 1 1] Quick Load
  (:Pressed
    (SaveGame|DoesSaveGameExist "BP_Game")
    (if true
      (bind _returnvalue (SaveGame|LoadGamefromSlot "BP_Game"))
      (bind _assave_info (Utilities|Casting|CastToSaveInfo _returnvalue))
      (Variables|Default|SetSaveInfoVar _assave_info)
      (Utilities|LoadGameVars)
      (Utilities|LoadTransforms))))

(fn ConstructionScript)

(fn PepperCollected
  (Variables|Default|SetScore (+ (Variables|Default|GetScore) (* (Variables|Default|GetLevel) 10)))
  (Variables|Default|SetPepperCount (+ (Variables|Default|GetPepperCount) 1))
  (if (== (Math|Integer|%(Integer) (Variables|Default|GetPepperCount) 5) 0)
    (Variables|Default|SetTime (+ (Variables|Default|GetTime) 15))
    (Variables|Default|SetLevel (Math|Integer|Min(Integer) (+ (Variables|Default|GetLevel) 1) 5))))